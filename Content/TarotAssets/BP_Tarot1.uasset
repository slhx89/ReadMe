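; Tarot card actor whose face is selected by U and V material parameters supplied by an NPC.
; The construction script creates a dynamic face material from the mesh's first material, with no step assigning it back to the mesh.
; BeginPlay copies the NPC's U and V once and binds to its card-call notification.
; The changecard event writes those stored values into the face material.
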(event Custom|change%20card
  (bind _dim_tarotface (Variables|Default|GetDIM_TarotFace))
  (Rendering|Material|SetScalarParameterValue _dim_tarotface "U" (Variables|Default|GetU) :!class /Script/Engine.MaterialInstanceDynamic)
  (Rendering|Material|SetScalarParameterValue _dim_tarotface "V" (Variables|Default|GetV) :!class /Script/Engine.MaterialInstanceDynamic))

(event EventBeginPlay
  (bind _npc (Variables|Default|GetNPC))
  (Variables|Default|SetU (Variables|/Game/MetaHumans/lexa/BP_lexa.BP_lexa_C|GetU _npc))
  (Variables|Default|SetV (Variables|/Game/MetaHumans/lexa/BP_lexa.BP_lexa_C|GetV _npc))
  (EventDispatchers|BindEventtoNotifyCardCall _npc (EventDispatchers|CreateEvent :!event Custom|change%20card)))

(event Collision|EventActorBeginOverlap
  (params (OtherActor :type Actor%20Object%20Reference)))

(event EventTick
  (params (DeltaSeconds :type Float%20%28single-precision%29)))

(fn ConstructionScript
  (bind _returnvalue (Rendering|Material|CreateDynamicMaterialInstance (Rendering|Material|GetMaterial (Variables|Default|GetStaticMesh) 0) "Face" "None" :!class /Script/Engine.KismetMaterialLibrary))
  (Variables|Default|SetDIM_TarotFace _returnvalue))